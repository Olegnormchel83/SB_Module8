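; BP_PowerUp is a moving power-up actor that displays its type on a text render component.
; The construction script selects PowerupType from a random index, though both options map to the same enum value, and writes its name to the text.
; Tick offsets the actor by Direction times Speed without sweeping, and overlapping a KillZVolume destroys it.
; No pickup effect is implemented in these graphs.
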(event `self.ReceiveActorBeginOverlap`
  (params (OtherActor :type "Actor Object Reference"))
  (cast `KillZVolume` OtherActor)
  (`self.K2_DestroyActor`))

(event `self.ReceiveTick`
  (params (DeltaSeconds :type "Float (single-precision)"))
  (`self.K2_AddActorWorldOffset` (* (* (`self.Direction`) (`self.Speed`)) DeltaSeconds)))

(fn `UserConstructionScript`
  (set `self.PowerupType` (select `int` (`KismetMathLibrary.RandomIntegerInRange` 0 1) :`0` "NewEnumerator0" :`1` "NewEnumerator0" :!type "/Game/Blueprints/Powerups/E_PowerupType Enum"))
  (`TextRenderComponent.K2_SetText` (`self.TextRender`) (`KismetTextLibrary.Conv_StringToText` (`|GetEnumeratorNameAsString` (`self.PowerupType`)))))