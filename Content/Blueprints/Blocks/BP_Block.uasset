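; BP_Block is a destructible block that can drop a powerup, apparently for a Breakout-style game.
; Hits from BP_Player subtract that actor's Damage from HP, swap the cube's material at exactly one HP and destroy the block at zero or below.
; Its OnDestroyed event runs a weighted chance roll that spawns a random double-ball, double-damage or carriage-size powerup at its location, chosen from a hardcoded class list.
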(event `self.ReceiveBeginPlay`
  (`parent.ReceiveBeginPlay`)
  (add `self.OnDestroyed` (delegate `SpawnPowerup`)))

(event `SpawnPowerup` :!signature `self.OnDestroyed`
  (params (DestroyedActor :type "Actor Object Reference"))
  (`self.RandomPowerup`))

(event `self.ReceiveActorBeginOverlap`
  (params (OtherActor :type "Actor Object Reference"))
  (`parent.ReceiveActorBeginOverlap` OtherActor))

(event `self.ReceiveTick`
  (params (DeltaSeconds :type "Float (single-precision)"))
  (`parent.ReceiveTick` DeltaSeconds))

(event `self.ReceiveHit`
  (params (MyComp :type "PrimitiveComponent Object Reference") (Other :type "Actor Object Reference") (OtherComp :type "PrimitiveComponent Object Reference") (bSelfMoved :type Boolean) (HitLocation :type "Vector Structure") (HitNormal :type "Vector Structure") (NormalImpulse :type "Vector Structure") (Hit :type "HitResult Structure (by ref)"))
  (bind _asbp_player (cast `/Game/Blueprints/Ball/BP_Player` Other))
  (set `self.HP` (- (`self.HP`) (`/Game/Blueprints/Ball/BP_Player.Damage` _asbp_player)))
  (if (== (`self.HP`) 1)
    (`PrimitiveComponent.SetMaterial` (`self.Cube`) 0 "/Game/Materials/EditorBrushMaterial.EditorBrushMaterial")
    (elif (<= (`self.HP`) 0)
      (`self.K2_DestroyActor`))))

(fn `RandomPowerup`
  (if (`KismetMathLibrary.RandomBoolWithWeight` (`self.SpawnPowerupChance`))
    (`|SpawnActorFromClass` (select `int` (`KismetMathLibrary.RandomInteger` 3) :`0` "/Game/Blueprints/Powerups/BP_DoubleBall.BP_DoubleBall_C" :`1` "/Game/Blueprints/Powerups/BP_DoubleDamage.BP_DoubleDamage_C" :`2` "/Game/Blueprints/Powerups/BP_CarriageSize.BP_CarriageSize_C" :!type "Actor Class Reference") (`KismetMathLibrary.MakeTransform` (`self.K2_GetActorLocation`)) "AlwaysSpawn" "OverrideRootScale" null null)))

(fn `UserConstructionScript`
  (`parent.UserConstructionScript`))