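; BP_Pawn is a player-controlled pawn that slides sideways and spawns the ball in play.
; The MoveLeftRightAD axis input applies a fixed, swept world Y offset by sign on each input event, with no delta-time scaling.
; On BeginPlay, SpawnBall spawns a BP_Player at the capsule's location, stores it as PlayingBall and binds an event to its OnDead dispatcher.
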(event `InputAxis|MoveLeftRightAD`
  (params (AxisValue :type "Float (single-precision)"))
  (if (< AxisValue 0.0)
    (`self.K2_AddActorWorldOffset` (0.0 -50.0 0.0) true)))

(event `InputAxis|MoveLeftRightAD`
  (params (AxisValue :type "Float (single-precision)"))
  (if (> AxisValue 0.0)
    (`self.K2_AddActorWorldOffset` (0.0 50.0 0.0) true)))

(event `self.ReceiveBeginPlay`
  (`self.SpawnBall`))

(event `self.ReceiveActorBeginOverlap`
  (params (OtherActor :type "Actor Object Reference")))

(event `self.ReceiveTick`
  (params (DeltaSeconds :type "Float (single-precision)")))

(fn `SpawnBall`
  (bind _returnvalue (`|SpawnActorFromClass` "/Game/Blueprints/BP_Player.BP_Player_C" (`KismetMathLibrary.MakeTransform` (`SceneComponent.K2_GetComponentLocation` (`self.Capsule`))) "AlwaysSpawn" "OverrideRootScale" null null))
  (bind _output_get (set `self.PlayingBall` _returnvalue))
  (add `/Game/Blueprints/BP_Player.OnDead` _output_get (`|CreateDelegate` :!event `SpawnBall`))
  (return))

(fn `UserConstructionScript`)